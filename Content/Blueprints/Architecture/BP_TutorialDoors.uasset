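; BP_TutorialDoors is a double door actor, named for the tutorial, that slides open when any actor overlaps it and then removes itself.
; Overlap caches each panel's relative location and calls OpenDoors, where two timelines lerp Left and Right in opposite directions along local Y.
; Each timeline's Update also feeds a two-second Delay, after which the panel is hidden and the whole actor destroyed.
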(event `self.ReceiveActorBeginOverlap`
  (params (OtherActor :type "Actor Object Reference"))
  (`|ExecutionSequence`
    (:`then_0`
      (set `self.LeftDoor` (`SceneComponent.RelativeLocation` (`self.Left`))))
    (:`then_1`
      (set `self.RightDoor` (`SceneComponent.RelativeLocation` (`self.Right`)))))
  (`self.OpenDoors`))

(event `OpenDoors`
  (bind _right (`self.Right`))
  (bind _leftdoor (`self.LeftDoor`))
  (bind _rightdoor (`self.RightDoor`))
  (bind _left (`self.Left`))
  (`|ExecutionSequence`
    (:`then_0`
      (bind (_direction _transition) (`Timeline|DoorAnimation`)
        (:`Update`
          (`SceneComponent.K2_SetRelativeLocation` _left (`KismetMathLibrary.VLerp` _leftdoor (+ _leftdoor (0.0 -200.0 0.0)) _transition) false false)
          (`KismetSystemLibrary.Delay` 2.0)
          (`SceneComponent.SetVisibility` _left false false))))
    (:`then_1`
      (bind (_direction_2 _transition_2) (`Timeline|Timeline`)
        (:`Update`
          (`SceneComponent.K2_SetRelativeLocation` _right (`KismetMathLibrary.VLerp` _rightdoor (+ _rightdoor (0.0 200.0 0.0)) _transition_2) false false)
          (`KismetSystemLibrary.Delay` 2.0)
          (`SceneComponent.SetVisibility` _right false false)))))
  (`self.K2_DestroyActor`))

(fn `UserConstructionScript`)