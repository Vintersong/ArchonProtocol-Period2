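; Architecture helper actor that lays out a straight row of repeated meshes, such as walls, as instances of one mesh.
; The construction script adds an Instanced Static Mesh component, assigns Mesh, then loops from zero to NumberOfWalls adding instances in local space.
; Each instance is offset by its index times Distance, along X or Y depending on UseXValue.
; The event graph has no active logic.
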(fn `UserConstructionScript`
  (bind _distance (`self.Distance`))
  (bind _returnvalue (`AddComponent|NODE_AddInstancedStaticMeshComponent-0`))
  (`StaticMeshComponent.SetStaticMesh` _returnvalue (`self.Mesh`))
  (for _index (range (+ (`self.Number of Walls`) 1))
    (if (`self.Use X Value`)
      (`InstancedStaticMeshComponent.AddInstance` _returnvalue (`KismetMathLibrary.MakeTransform` (`KismetMathLibrary.MakeVector` (`KismetMathLibrary.Conv_IntToDouble` (* _index _distance)))) false)
      (else
        (`InstancedStaticMeshComponent.AddInstance` _returnvalue (`KismetMathLibrary.MakeTransform` (`KismetMathLibrary.MakeVector` 0.0 (`KismetMathLibrary.Conv_IntToDouble` (* _index _distance)))) false)))))