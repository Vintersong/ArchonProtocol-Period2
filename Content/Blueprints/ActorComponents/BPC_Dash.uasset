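; Actor component that gives the owning BP_ThirdPersonCharacter a forward dash with a cooldown.
; Dash launches the character along its facing direction by DashDistance, overriding current velocity, and lowers braking friction, which is never restored here.
; A fixed timer calls ResetDash to re-enable dashing, with debug prints marking cooldown start and end.
; CheckDash uses a DoOnce to seed CanDash from DashActive on the first dash attempt.
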(event `self.ReceiveBeginPlay`
  (`self.SetActive` true)
  (set `self.OwnerActor` (cast `/Game/ThirdPerson/Blueprints/BP_ThirdPersonCharacter` (`self.GetOwner`) :!pure true)))

(event `Check Dash`
  (`/Engine/EditorBlueprintResources/StandardMacros.DoOnce` false
    (:`Completed`
      (set `self.CanDash` (`self.DashActive?`)))))

(event `Dash`
  (`self.Check Dash`)
  (set `self.IsDashing?` true)
  (if (`self.CanDash`)
    (if (`self.IsDashing?`)
      (`Character.LaunchCharacter` (`self.OwnerActor`) (* (`KismetMathLibrary.GetForwardVector` (`Actor.K2_GetActorRotation` (`self.GetOwner`))) (`self.DashDistance`)) true true)
      (set `CharacterMovementComponent.BrakingFriction` 0.1 (`Character.CharacterMovement` (`self.OwnerActor`)))
      (`KismetSystemLibrary.K2_SetTimerDelegate` (delegate `ResetDash`) 2.0)
      (set `self.CanDash` false)
      (`KismetSystemLibrary.PrintString` "On Cooldown!"))))

(event `ResetDash`
  (set `self.CanDash` true)
  (set `self.IsDashing?` false)
  (`KismetSystemLibrary.PrintString` "Off Cooldown!"))