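; Teleport trigger that moves the player between the main level and the double jump tutorial level.
; On overlap it plays a sound, spawns an attached particle effect at its box and hides the player character's mesh.
; When the effect finishes, it reads the level index from BP_LevelMarker and opens _main for index 1, otherwise _doubleJump.
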(event `self.ReceiveBeginPlay`)

(event `LoadLevel`
  (if (== (`self.LevelIndexNumber`) 1)
    (`GameplayStatics.OpenLevel` "_main")
    (else
      (`GameplayStatics.OpenLevel` "_doubleJump"))))

(event `self.ReceiveActorBeginOverlap`
  (params (OtherActor :type "Actor Object Reference"))
  (bind _asbp_third_person_character (cast `/Game/ThirdPerson/Blueprints/BP_ThirdPersonCharacter` OtherActor :!pure true))
  (`self.PlaySound`)
  (`self.Effects`)
  (set `self.Player` _asbp_third_person_character)
  (`SceneComponent.SetVisibility` (`Character.Mesh` _asbp_third_person_character) false false)
  (`KismetSystemLibrary.PrintString` (`self.DoubleJump`)))

(event `Effects`
  (bind _returnvalue (`NiagaraFunctionLibrary.SpawnSystemAttached` (`self.VFX`) (`self.Box`) "None" (`self.K2_GetActorLocation`) (struct) "KeepWorldPosition"))
  (`/Engine/EditorBlueprintResources/StandardMacros.IsValid` _returnvalue
    (:`Is Valid`
      (add `NiagaraComponent.OnSystemFinished` _returnvalue (delegate `Teleport`)))))

(event `Teleport`
  (params (PSystem :type "NiagaraComponent Object Reference"))
  (bind _returnvalue (`GameplayStatics.GetActorOfClass` "/Game/Blueprints/TutorialBPs/LevelMarkers/BP_LevelMarker.BP_LevelMarker_C"))
  (set `self.LevelIndexNumber` (`/Game/Blueprints/TutorialBPs/LevelMarkers/BP_LevelMarker.LevelIndex` _returnvalue))
  (`self.LoadLevel`))

(event `PlaySound`
  (`GameplayStatics.PlaySoundAtLocation` (`self.SoundCue`) (`self.K2_GetActorLocation`) (struct) 1.0 1.0 0.0 null null null null))

(fn `UserConstructionScript`)