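; BP_Tutorial_Dash is an overlap-triggered actor that switches levels in the dash tutorial.
; On overlap it casts the other actor to BP_ThirdPersonCharacter, prints its name, and reads LevelIndex from the BP_LevelMarker_dash found in the world.
; LoadLevel then opens "_main" when that index is 2, and "_dash" otherwise.
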(event `self.ReceiveActorBeginOverlap`
  (params (OtherActor :type "Actor Object Reference"))
  (bind _output_get (set `self.Player` (cast `/Game/ThirdPerson/Blueprints/BP_ThirdPersonCharacter` OtherActor :!pure true)))
  (`KismetSystemLibrary.PrintString` (`KismetSystemLibrary.GetDisplayName` _output_get))
  (bind _returnvalue (`GameplayStatics.GetActorOfClass` "/Game/Blueprints/TutorialBPs/LevelMarkers/BP_LevelMarker_dash.BP_LevelMarker_dash_C"))
  (set `self.LevelIndexNumber` (`/Game/Blueprints/TutorialBPs/LevelMarkers/BP_LevelMarker.LevelIndex` _returnvalue))
  (`self.LoadLevel`))

(event `LoadLevel`
  (if (== (`self.LevelIndexNumber`) 2)
    (`GameplayStatics.OpenLevel` "_main")
    (else
      (`GameplayStatics.OpenLevel` "_dash"))))

(fn `UserConstructionScript`)